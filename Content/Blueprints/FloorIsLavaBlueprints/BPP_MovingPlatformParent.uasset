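; Parent Blueprint for moving platforms, apparently for a Floor Is Lava mode, that slides a static mesh back and forth.
; BeginPlay starts the Movement timeline at the Speed play rate, scaling its Distance track by horizontal (X) and vertical (Z) distances for a swept relative move.
; A Pause delay chained to the timeline's Update, rather than Finished, then toggles IsLooped to alternate Play and Reverse.
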(event `self.ReceiveBeginPlay`
  (`TimelineComponent.SetPlayRate` (`self.Movement`) (`self.Speed`))
  (bind (_direction _distance) (`Timeline|Movement` :!label _label)
    (:`Update`
      (`SceneComponent.K2_SetRelativeLocation` (`self.StaticMesh`) (`KismetMathLibrary.MakeVector` (* _distance (`self.HorizontalDistance`)) 0.0 (* _distance (`self.VerticalDistance`))) true false)
      (`KismetSystemLibrary.Delay` (`self.Pause`))
      (if (`self.IsLooped`)
        (set `self.IsLooped` false)
        (goto _label :!via `Reverse`)
        (else
          (set `self.IsLooped` true)
          (goto _label))))))

(fn `UserConstructionScript`)