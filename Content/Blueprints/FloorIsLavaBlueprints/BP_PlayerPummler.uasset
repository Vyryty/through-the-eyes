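; BP_PlayerPummler spawns random actors around the player and launches them at the player's position, once every ThrowDelay via a Delay on Tick.
; Spawn points use a random cone opposite the camera's forward, sized outside its FOV, with random distance and fixed height offset.
; Each actor from the Throwables array gets a runtime ProjectileMovementComponent, with velocity from SuggestProjectileVelocityMovingTarget using TimeToTarget as flight time.
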(event `self.ReceiveTick`
  (params (DeltaSeconds :type "Float (single-precision)"))
  (bind _returnvalue (`GameplayStatics.GetPlayerCameraManager` 0))
  (bind _throwspawnlocation_location (`KismetMathLibrary.BreakTransform` (`self.ThrowSpawnLocation`)))
  (bind _returnvalue_2 (`KismetMathLibrary.RandomFloatInRange` (`self.ThrowDistanceMin`) (`self.ThrowDistanceMax`)))
  (bind (_returnvalue_x _returnvalue_y) (`KismetMathLibrary.BreakVector` (`self.GetActorForwardVector` _returnvalue)))
  (bind _returnvalue_location (`KismetMathLibrary.BreakTransform` (`self.GetTransform` (`GameplayStatics.GetPlayerCharacter` 0))))
  ;[1 1 1] Throws Every Throw Delay
  (`KismetSystemLibrary.Delay` (`self.ThrowDelay`))
  (bind _output_get (set `self.ThrowSpawnLocation` (`KismetMathLibrary.MakeTransform` (+ (+ (* (`KismetMathLibrary.RandomUnitVectorInEllipticalConeInDegrees` (`KismetMathLibrary.NegateVector` (`KismetMathLibrary.MakeVector` _returnvalue_x _returnvalue_y)) (/ (- 360.0 (`PlayerCameraManager.GetFOVAngle` _returnvalue)) 2.0) 20.0) (`KismetMathLibrary.MakeVector` _returnvalue_2 _returnvalue_2)) (`KismetMathLibrary.MakeVector` 0.0 0.0 (`self.ThrowHeight`))) _returnvalue_location))))
  ;[1 1 1] Throws a random Throwable (Must be added to array)
  (bind _returnvalue_3 (`|SpawnActorFromClass` (`KismetArrayLibrary.Array_Random` (`self.Throwables`)) _output_get "Undefined" "MultiplyWithRoot" null null))
  ;[1 1 1] Throws the Throwable at the player, with a specified air time (Time To Target)
  (bind _outlaunchvelocity (`GameplayStatics.SuggestProjectileVelocity_MovingTarget` _throwspawnlocation_location _returnvalue_3 (- (`self.K2_GetActorLocation` (`GameplayStatics.GetPlayerCharacter` 0)) _throwspawnlocation_location) 0.0 (`self.Time to Target`) "None"))
  (bind _returnvalue_4 (`AddComponent|NODE_AddProjectileMovementComponent-0` :`self` _returnvalue_3))
  (set `MovementComponent.Velocity` _outlaunchvelocity _returnvalue_4))

(fn `UserConstructionScript`)