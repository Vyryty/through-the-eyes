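; BP_Fallable is a Floor Is Lava actor whose static mesh falls and then sinks after a character hits it.
; The first Character hit triggers a DoOnce, then a delay leads into the Fall timeline, followed by a second delay and the Sink timeline.
; Both timelines drive the mesh's relative Z through distance curves, with configurable delays, play rates and distances, and Sink offsets by the fall distance.
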(event `self.ReceiveHit`
  (params (MyComp :type "PrimitiveComponent Object Reference") (Other :type "Actor Object Reference") (OtherComp :type "PrimitiveComponent Object Reference") (bSelfMoved :type Boolean) (HitLocation :type "Vector Structure") (HitNormal :type "Vector Structure") (NormalImpulse :type "Vector Structure") (Hit :type "HitResult Structure (by ref)"))
  (cast `Character` Other)
  (`/Engine/EditorBlueprintResources/StandardMacros.DoOnce` false
    (:`Completed`
      (`KismetSystemLibrary.Delay` (`self.FallDelay`))
      (`TimelineComponent.SetPlayRate` (`self.Fall`) (`self.FallSpeed`))
      (bind (_direction _distance) (`Timeline|Fall`)
        (:`Update`
          (`SceneComponent.K2_SetRelativeLocation` (`self.StaticMesh`) (`KismetMathLibrary.MakeVector` 0.0 0.0 (* _distance (`self.FallDistance`))) false false))
        (:`Finished`
          (`KismetSystemLibrary.Delay` (`self.SinkDelay`))
          (`TimelineComponent.SetPlayRate` (`self.Sink`) (`self.SinkSpeed`))
          (bind (_direction_2 _distance_2) (`Timeline|Sink`)
            (:`Update`
              (`SceneComponent.K2_SetRelativeLocation` (`self.StaticMesh`) (`KismetMathLibrary.MakeVector` 0.0 0.0 (- (* _distance_2 (`self.SinkDistance`)) (`self.FallDistance`))) false false))))))))

(fn `UserConstructionScript`)