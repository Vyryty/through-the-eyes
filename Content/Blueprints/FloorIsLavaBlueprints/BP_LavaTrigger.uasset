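; Lava kill trigger for the Floor Is Lava blueprints that shows a death screen when a Character enters its box.
; While CanKill is set, the box overlap adds WG_LavaDeathScreen to the viewport and stops the current line on BP_DialogueHandler.
; The trigger does not destroy or respawn the character, and its blackscreen, audio and delay placeholders are unconnected debug prints.
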(event `self.Box.OnComponentBeginOverlap`
  (params (OverlappedComponent :type "PrimitiveComponent Object Reference") (OtherActor :type "Actor Object Reference") (OtherComp :type "PrimitiveComponent Object Reference") (OtherBodyIndex :type Integer) (bFromSweep :type Boolean) (SweepResult :type "HitResult Structure (by ref)"))
  (if (`self.CanKill`)
    (cast `Character` OtherActor)
    (`KismetSystemLibrary.PrintString` "Die")
    (bind _returnvalue (`|CreateWidget` "/Game/UI/WG_LavaDeathScreen.WG_LavaDeathScreen_C"))
    (`UserWidget.AddToViewport` _returnvalue 0)
    (bind _returnvalue_2 (`GameplayStatics.GetActorOfClass` "/Game/Blueprints/UI_Blueprints/BP_DialogueHandler.BP_DialogueHandler_C"))
    (`AudioComponent.Stop` (`/Game/Blueprints/UI_Blueprints/BP_DialogueHandler.CurrentLineRef` _returnvalue_2))))

(fn `UserConstructionScript`)