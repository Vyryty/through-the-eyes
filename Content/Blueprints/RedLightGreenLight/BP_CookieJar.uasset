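; BP_CookieJar is the goal and round controller for a Red Light, Green Light game, printing a win when the player overlaps its capsule.
; Once Alert starts an opening lit phase, Tick alternates randomly timed dark and lit phases through BP_LightSystem.
; Moving while illuminated, detected by per-frame squared distance against a threshold, drains a leeway timer that resets each dark phase; movement after it empties loses.
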(event `self.ReceiveBeginPlay`
  (bind _outactors (`GameplayStatics.GetAllActorsOfClass` "/Game/Blueprints/_Templates/BP_FirstPersonCharacter.BP_FirstPersonCharacter_C"))
  (set `self.Player` (`|GetArrayItem` _outactors))
  (bind _outactors_2 (`GameplayStatics.GetAllActorsOfClass` "/Game/Blueprints/RedLightGreenLight/BP_LightSystem.BP_LightSystem_C"))
  (set `self.Lights` (`|GetArrayItem` _outactors_2)))

(event `Alert`
  (set `self.Begun` true)
  (`self.Change State` 2))

(event `self.ReceiveTick`
  (params (DeltaSeconds :type "Float (single-precision)"))
  (bind _rlduration (`self.RLDuration`))
  (bind _leeway_timer (`self.Leeway Timer`))
  (bind _state (`self.State`))
  (bind _timer (`self.Timer`))
  (if (and (`self.Begun`) (`self.Game Going`))
    (`|ExecutionSequence`
      (:`then_0`
        (if (`self.Start of State`)
          (set `self.Start of State` false)
          (`/Game/Blueprints/RedLightGreenLight/BP_LightSystem.Power Lights` (`self.Lights`) (!= 0 _state) (select `int` _state :`0` 4.0 :`1` _rlduration :`2` _rlduration) (select `int` _state :`0` 0.475 :`1` 0.625 :`2` 0.475))))
      (:`then_1`
        (if (<= _timer 0.0)
          (`self.Change State` (`KismetMathLibrary.SelectInt` 0 1 (!= _state 0)))
          (else
            (set `self.Timer` (- _timer DeltaSeconds)))))
      (:`then_2`
        (if (and (`self.Player Moving`) (`/Game/Blueprints/RedLightGreenLight/BP_LightSystem.Player Illuminated` (`self.Lights`)))
          (if (<= _leeway_timer 0.0)
            (set `self.Game Going` false)
            (`KismetSystemLibrary.PrintString` "You lose!")
            (else
              (set `self.Leeway Timer` (- _leeway_timer DeltaSeconds)))))))))

(event `self.Capsule.OnComponentBeginOverlap`
  (params (OverlappedComponent :type "PrimitiveComponent Object Reference") (OtherActor :type "Actor Object Reference") (OtherComp :type "PrimitiveComponent Object Reference") (OtherBodyIndex :type Integer) (bFromSweep :type Boolean) (SweepResult :type "HitResult Structure (by ref)"))
  (cast `/Game/Blueprints/_Templates/BP_FirstPersonCharacter` OtherActor)
  (`KismetSystemLibrary.PrintString` "You win!"))

(fn `Change State`
  (params (`New State` :type Integer))
  (bind _returnvalue (`KismetMathLibrary.RandomFloatInRange` (`self.MinRLDuration`) (`self.MaxRLDuration`)))
  (bind _output_get (set `self.State` `New State`))
  (set `self.Start of State` true)
  (set `self.Timer` (select `int` _output_get :`0` (`KismetMathLibrary.RandomFloatInRange` (`self.MinGLTime`) (`self.MaxGLTime`)) :`1` _returnvalue :`2` _returnvalue))
  (if (== _output_get 0)
    (set `self.Leeway Timer` (`self.RLLeeway`))))

(fn `Player Moving`
  (returns (`Player Moving` :type Boolean))
  (locals (Result :type Boolean) (Threshold :type "Float (double-precision)" :default 0.25))
  (bind _returnvalue (`SceneComponent.K2_GetComponentLocation` (`Character.CapsuleComponent` (`self.Player`))))
  (bind _output_get (set `local.Result` (> (`KismetMathLibrary.Vector_DistanceSquared` _returnvalue (`self.Prev Player Location`)) (`local.Threshold`))))
  (set `self.Prev Player Location` _returnvalue)
  (return _output_get))

(fn `UserConstructionScript`)