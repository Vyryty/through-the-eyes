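; Light controller for the Red Light Green Light game that switches a set of placed lights and reports whether the player is illuminated.
; At BeginPlay it caches each light's original intensity in a map, applies the starting state and finds the player character.
; PowerLights zeroes or restores intensities, staggering switches with a Delay loop until the time budget runs out.
; PlayerIlluminated judges by whether the light nearest the player is on, using squared distances.
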(event `self.ReceiveBeginPlay`
  (for _array_element (`self.Light References`)
    (bind _lightcomponent (`Light.LightComponent` _array_element))
    (`BlueprintMapLibrary.Map_Add` (`self.Lights`) _lightcomponent (`LightComponentBase.Intensity` _lightcomponent)))
  (`self.Power Lights` (`self.Start On`))
  (bind _outactors (`GameplayStatics.GetAllActorsOfClass` "/Game/Blueprints/_Templates/BP_FirstPersonCharacter.BP_FirstPersonCharacter_C"))
  (set `self.Player` (`|GetArrayItem` _outactors)))

(event `Power Lights`
  (params (`Turn On` :type Boolean) (`Max Time` :type "Float (double-precision)") (`Light Delay` :type "Float (double-precision)" :default 0.625))
  (bind _lights (`self.Lights`))
  (bind _returnvalue (- (`self.Power Time`) `Light Delay`))
  (set `self.Power Time` `Max Time`)
  (bind _keys (`BlueprintMapLibrary.Map_Keys` _lights))
  (bind _output_get (set `self.Index` 0))
  (if (< _output_get (`KismetArrayLibrary.Array_Length` _keys)) :!label _label
    (bind _output (`|GetArrayItem` _keys (`self.Index`)))
    (`LightComponent.SetIntensity` _output (`KismetMathLibrary.SelectFloat` (`BlueprintMapLibrary.Map_Find` _lights _output) 0.0 `Turn On`))
    (`/Engine/EditorBlueprintResources/StandardMacros.IncrementInt` (`self.Index`)
      (:`  `
        (if (> _returnvalue 0.0)
          (`KismetSystemLibrary.Delay` `Light Delay`)
          (set `self.Power Time` _returnvalue)
          (goto _label)
          (else
            (goto _label)))))))

(fn `Player Illuminated`
  (returns (Output :type Boolean))
  (locals (`Closest Dist` :type "Float (double-precision)" :default 3753136614371145.5) (Result :type Boolean))
  (bind _keys (`BlueprintMapLibrary.Map_Keys` (`self.Lights`)))
  (for _array_element _keys
    (bind _returnvalue (`KismetMathLibrary.Vector_DistanceSquared` (`SceneComponent.K2_GetComponentLocation` _array_element) (`SceneComponent.K2_GetComponentLocation` (`Character.CapsuleComponent` (`self.Player`)))))
    (if (<= _returnvalue (`local.Closest Dist`))
      (set `local.Closest Dist` _returnvalue)
      (set `local.Result` (> (`LightComponentBase.Intensity` _array_element) 0.0))))
  (return (`local.Result`)))

(fn `UserConstructionScript`)