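; BP_NoisyThing is a trap actor in the RedLightGreenLight game that makes noise and alerts "Dad" when the first-person player overlaps its box.
; On BeginPlay it stores the first BP_CookieJar in the level as the Dad reference.
; An overlap while active calls Alert on Dad, plays a reverb fart sound, then after a half-second delay calls the empty Deactivate function and clears the Active flag.
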(event `self.ReceiveBeginPlay`
  (bind _outactors (`GameplayStatics.GetAllActorsOfClass` "/Game/Blueprints/RedLightGreenLight/BP_CookieJar.BP_CookieJar_C"))
  (set `self.Dad` (`|GetArrayItem` _outactors)))

(event `self.Box.OnComponentBeginOverlap`
  (params (OverlappedComponent :type "PrimitiveComponent Object Reference") (OtherActor :type "Actor Object Reference") (OtherComp :type "PrimitiveComponent Object Reference") (OtherBodyIndex :type Integer) (bFromSweep :type Boolean) (SweepResult :type "HitResult Structure (by ref)"))
  (if (`self.Active`)
    (cast `/Game/Blueprints/_Templates/BP_FirstPersonCharacter` OtherActor)
    (`/Game/Blueprints/RedLightGreenLight/BP_CookieJar.Alert` (`self.Dad`))
    (`GameplayStatics.SpawnSound2D` "/Game/Sound/SoundFX/fart-with-reverb.fart-with-reverb" 1.0 1.0 0.0 null)
    (`KismetSystemLibrary.Delay` 0.5)
    (`self.Deactivate`)
    (set `self.Active` false)))

(fn `Deactivate`)

(fn `UserConstructionScript`)