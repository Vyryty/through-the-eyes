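; BP_DialogueHandler is an actor that plays random dialogue lines as 2D sounds at random intervals.
; Tick accumulates time and, once past the chosen wait, resets it, spawns the queued line and stores its audio reference.
; After a delay matching the line's duration, RanDialogueAndTime picks the next line and whole-second wait, printing the line's name.
; The timer keeps counting during playback, so waits are measured from each line's start.
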(event `self.ReceiveBeginPlay`
  (`self.RanDialogueAndTime`))

(event `self.ReceiveTick`
  (params (DeltaSeconds :type "Float (single-precision)"))
  (bind _nextdialogue (`self.NextDialogue`))
  ;[1 1 1] Checking and Playing
  (bind _output_get (set `self.TimeSinceLastLine` (+ DeltaSeconds (`self.TimeSinceLastLine`))))
  (`/Engine/EditorBlueprintResources/StandardMacros.CompareFloat` _output_get (`KismetMathLibrary.Conv_IntToDouble` (`self.TimeToNextLine`))
    (:`>`
      (if true
        (set `self.TimeSinceLastLine` 0.0)
        (bind _returnvalue (`GameplayStatics.SpawnSound2D` _nextdialogue 1.0 1.0 0.0 null))
        (set `self.CurrentLineRef` _returnvalue)
        (`KismetSystemLibrary.Delay` (`SoundBase.Duration` _nextdialogue))
        (`self.RanDialogueAndTime`)))))

(event `RanDialogueAndTime`
  ;[1 1 1] Randomizing Time and Dialogue Line
  (set `self.TimeToNextLine` (`KismetMathLibrary.RandomIntegerInRange` (`self.MinTime`) (`self.MaxTime`)))
  (bind _output_get (set `self.DialogueLineLength` (`KismetArrayLibrary.Array_Length` (`self.DialogueLines`))))
  (bind _result (`/Engine/EditorBlueprintResources/StandardMacros.DecrementInt` _output_get)
    (:`  `
      (bind _output_get_2 (set `self.NextDialogue` (`|GetArrayItem` (`self.DialogueLines`) (`KismetMathLibrary.RandomIntegerInRange` 0 _result))))
      (`KismetSystemLibrary.PrintString` (`KismetSystemLibrary.GetDisplayName` _output_get_2)))))

(fn `UserConstructionScript`)