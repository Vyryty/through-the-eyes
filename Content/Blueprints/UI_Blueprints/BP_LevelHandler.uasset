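; BP_LevelHandler sets up and manages a level's music and base HUD.
; On BeginPlay it spawns the level music as a persistent 2D sound, creates the current task, crosshair and dialogue widgets, then shows the beginning task.
; Events pause, resume or fade out the music through the stored audio component.
; Other events forward task and dialogue text updates, including a dialogue clear, to the widgets.
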(event `PauseMusic`
  ;[1 1 1] Handling Music in Level
  (`AudioComponent.SetPaused` (`self.LevelMusicComp`) true))

(event `BeginMusic`
  ;[1 1 1] Handling Music in Level
  (bind _returnvalue (`GameplayStatics.SpawnSound2D` (`self.LevelMusic`) 1.0 1.0 0.0 null true))
  (bind _output_get (set `self.LevelMusicComp` _returnvalue))
  (`AudioComponent.AdjustVolume` _output_get 0.0 (`self.BaseVolumeLevel`) "Linear"))

(event `ResumeMusic`
  ;[1 1 1] Handling Music in Level
  (`AudioComponent.SetPaused` (`self.LevelMusicComp`) false))

(event `self.ReceiveBeginPlay`
  (`|ExecutionSequence`
    (:`then_0`
      (`self.BeginMusic`))
    (:`then_1`
      (`self.BuildUI`))
    (:`then_2`
      (`self.SetBeginningTask` ""))))

(event `StopMusic`
  ;[1 1 1] Handling Music in Level
  (`AudioComponent.FadeOut` (`self.LevelMusicComp`) (`self.MusicFadeEnd`) 0.0 "Linear"))

(event `UpdateTask`
  (params (InText :type Text))
  ;[1 1 1] Updating Task
  (`/Game/UI/WG_CurrentTask.UpdateCurrentTask` (stale `CreateCurrentTaskUI` _returnvalue) InText))

(event `BuildUI`
  ;[1 1 1] Separated In Case Need to Change or Delete Items
  ;;[1 1 1] Building Base UI For All Levels
  (`|ExecutionSequence`
    (:`then_0`
      (`self.CreateCurrentTaskUI`))
    (:`then_1`
      (`self.CreateCrosshair`))
    (:`then_2`
      (`self.CreateDialogueBox`))))

(event `SetBeginningTask`
  (params (InText :type Text))
  ;[1 1 1] Updating Task
  (`/Game/UI/WG_CurrentTask.UpdateCurrentTask` (stale `CreateCurrentTaskUI` _returnvalue) (`self.BeginningTask`)))

(event `CreateCurrentTaskUI`
  ;[1 1 1] Separated In Case Need to Change or Delete Items
  ;;[1 1 1] Creating the UI Widgets
  (bind _returnvalue (`|CreateWidget` "/Game/UI/WG_CurrentTask.WG_CurrentTask_C"))
  (`UserWidget.AddToViewport` _returnvalue 0))

(event `UpdateDialogue`
  (params (InText :type "Text (by ref)"))
  ;[1 1 1] Updating Dialogue
  (`/Game/UI/WG_Dialogue.UpdateCurrentDialogue` (stale `CreateDialogueBox` _returnvalue) InText false))

(event `CreateCrosshair`
  ;[1 1 1] Separated In Case Need to Change or Delete Items
  ;;[1 1 1] Creating the UI Widgets
  (bind _returnvalue (`|CreateWidget` "/Game/UI/WG_Crosshair.WG_Crosshair_C"))
  (`UserWidget.AddToViewport` _returnvalue 0))

(event `ClearDialogue`
  ;[1 1 1] Updating Dialogue
  (`/Game/UI/WG_Dialogue.UpdateCurrentDialogue` (stale `CreateDialogueBox` _returnvalue) (`self.ClearDialogueText`) true))

(event `CreateDialogueBox`
  ;[1 1 1] Separated In Case Need to Change or Delete Items
  ;;[1 1 1] Creating the UI Widgets
  (bind _returnvalue (`|CreateWidget` "/Game/UI/WG_Dialogue.WG_Dialogue_C"))
  (`UserWidget.AddToViewport` _returnvalue 0))

(fn `UserConstructionScript`)