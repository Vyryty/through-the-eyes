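; Game instance that keeps track of the current level and controls menu music across level loads.
; SetCurrentLevel maps CurrentLevelIndex to a level reference for the main menu, bedroom, living room, hallway or credits.
; RestartLevel reopens that stored level.
; Menu music events spawn or stop a 2D sound, using a MusicPlaying flag so it never starts twice.
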(event `RestartLevel`
  (`GameplayStatics.OpenLevelBySoftObjectPtr` (`self.PlayerCurrentLevel`)))

(event `PlayMenuMusic`
  (if (not (`self.MusicPlaying`))
    (bind _returnvalue (`GameplayStatics.SpawnSound2D` "/Game/Sound/Music/A_I_spy___.A_I_spy___" 1.0 1.0 0.0 null true))
    (set `self.Music` _returnvalue)
    (set `self.MusicPlaying` true)))

(event `StopMenuMusic`
  (`AudioComponent.Stop` (`self.Music`))
  (set `self.MusicPlaying` false))

(fn `SetCurrentLevel`
  (switch `int` (`self.CurrentLevelIndex`)
    (:`0`
      (set `self.PlayerCurrentLevel` "/Game/Levels/LVL_MainMenu.LVL_MainMenu"))
    (:`1`
      (set `self.PlayerCurrentLevel` "/Game/Levels/Bedroom/Bedroom_Base.Bedroom_Base"))
    (:`2`
      (set `self.PlayerCurrentLevel` "/Game/Levels/LivingRoom/Livingroom_Base.Livingroom_Base"))
    (:`3`
      (set `self.PlayerCurrentLevel` "/Game/Levels/Hallway/Hallway_Base.Hallway_Base"))
    (:`4`
      (set `self.PlayerCurrentLevel` "/Game/Levels/LVL_Credits.LVL_Credits"))))