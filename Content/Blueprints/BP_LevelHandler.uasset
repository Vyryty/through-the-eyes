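; BP_LevelHandler is a per-level manager actor that starts the level music and builds the base HUD on BeginPlay.
; It spawns LevelMusic as a 2D sound and keeps the component so PauseMusic and ResumeMusic events can toggle it.
; BuildUI creates current task, crosshair and dialogue box widgets in separate events and adds them to the viewport.
; UpdateTask forwards new text to the current task widget.
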(event `PauseMusic`
  ;[1 1 1] Handling Music in Level
  (`AudioComponent.SetPaused` (stale `BeginMusic` _returnvalue) true))

(event `self.ReceiveBeginPlay`
  (`|ExecutionSequence`
    (:`then_0`
      (`self.BeginMusic`))
    (:`then_1`
      (`self.BuildUI`))))

(event `BeginMusic`
  ;[1 1 1] Handling Music in Level
  (bind _returnvalue (`GameplayStatics.SpawnSound2D` (`self.LevelMusic`) 1.0 1.0 0.0 null)))

(event `ResumeMusic`
  ;[1 1 1] Handling Music in Level
  (`AudioComponent.SetPaused` (stale `BeginMusic` _returnvalue) false))

(event `UpdateTask`
  (params (InText :type Text))
  (`/Game/UI/WG_CurrentTask.UpdateCurrentTask` (stale `CreateCurrentTaskUI` _returnvalue) InText))

(event `BuildUI`
  ;[1 1 1] Separated In Case Need to Change or Delete Items
  ;;[1 1 1] Building Base UI For All Levels
  (`|ExecutionSequence`
    (:`then_0`
      (`self.CreateCurrentTaskUI`))
    (:`then_1`
      (`self.CreateCrosshair`))
    (:`then_2`
      (`self.CreateDialogueBox`))))

(event `CreateCurrentTaskUI`
  ;[1 1 1] Separated In Case Need to Change or Delete Items
  ;;[1 1 1] Creating the UI Widgets
  (bind _returnvalue (`|CreateWidget` "/Game/UI/WG_CurrentTask.WG_CurrentTask_C"))
  (`UserWidget.AddToViewport` _returnvalue 0))

(event `CreateCrosshair`
  ;[1 1 1] Separated In Case Need to Change or Delete Items
  ;;[1 1 1] Creating the UI Widgets
  (bind _returnvalue (`|CreateWidget` "/Game/UI/WG_Crosshair.WG_Crosshair_C"))
  (`UserWidget.AddToViewport` _returnvalue 0))

(event `CreateDialogueBox`
  ;[1 1 1] Separated In Case Need to Change or Delete Items
  ;;[1 1 1] Creating the UI Widgets
  (bind _returnvalue (`|CreateWidget` "/Game/UI/WG_Dialogue.WG_Dialogue_C"))
  (`UserWidget.AddToViewport` _returnvalue 0))

(fn `UserConstructionScript`)